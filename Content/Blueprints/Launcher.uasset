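; Launcher actor that lets the player fire projectiles while standing inside its trigger box.
; Entering or leaving the box toggles the prompt text's visibility and enables or disables input for the first player controller.
; Pressing Interact spawns a Projectile actor at the Cube component's world location and rotation.
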(event `self.ReceiveBeginPlay`)

(event `self.Box.OnComponentBeginOverlap`
  (params (OtherActor :type "Actor Object Reference") (OtherComp :type "PrimitiveComponent Object Reference") (OtherBodyIndex :type Integer) (bFromSweep :type Boolean) (SweepResult :type "HitResult Structure (by ref)"))
  ;[1 1 1] Collision enables input and text
  (`SceneComponent.ToggleVisibility` (`self.TextRender`) false)
  (`self.EnableInput` (`GameplayStatics.GetPlayerController` 0)))

(event `self.ReceiveActorBeginOverlap`
  (params (OtherActor :type "Actor Object Reference")))

(event `self.ReceiveTick`
  (params (DeltaSeconds :type "Float (single-precision)")))

(event `InputAction|Interact`
  (bind _cube (`self.Cube`))
  ;[1 1 1] Click activates Projectile Class
  (:`Pressed`
    (`|SpawnActorFromClass` "/Game/Blueprints/Projectile.Projectile_C" (`KismetMathLibrary.MakeTransform` (`SceneComponent.K2_GetComponentLocation` _cube) (`SceneComponent.K2_GetComponentRotation` _cube)))))

(event `self.Box.OnComponentEndOverlap`
  (params (OtherActor :type "Actor Object Reference") (OtherComp :type "PrimitiveComponent Object Reference") (OtherBodyIndex :type Integer))
  ;[1 1 1] Leaving Collision Disables Input and Text
  (`SceneComponent.ToggleVisibility` (`self.TextRender`) false)
  (`self.DisableInput` (`GameplayStatics.GetPlayerController` 0)))

(fn `UserConstructionScript`)
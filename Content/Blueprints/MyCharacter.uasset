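; Player character with camera-relative movement, mouse and gamepad look, energy-draining jumps, and projectile shooting with camera shake and sound.
; BeginPlay creates the GameHUD widget, which gates the inventory menu toggle and the five-item pickup limit.
; Pickups go through the PickUpItem dispatcher, and DropAction restores dropped actors at DropLocation.
; Holding slow-mo sets a flag that Tick turns into a slomo console command, and steps the camera FOV.
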(event `InputAxis|MoveForward`
  (params (AxisValue :type "Float (single-precision)"))
  ;[1 1 1] Charcter Movement
  (`self.AddMovementInput` (`KismetMathLibrary.GetForwardVector` (`KismetMathLibrary.MakeRot` 0.0 (.yaw (`self.GetControlRotation`)))) AxisValue))

(event `InputAxis|LookUp`
  (params (AxisValue :type "Float (single-precision)"))
  ;[1 1 1] Mouse Rotation'
  (`self.AddControllerPitchInput` AxisValue))

(event `InputAction|Jump`
  ;[1 1 1] Jumping
  (:`Pressed`
    (`self.Jump`)
    (set `self.Energy` (- (`self.Energy`) 0.05))))

(event `InputAxis|LookRight`
  (params (AxisValue :type "Float (single-precision)"))
  ;[1 1 1] Mouse Rotation'
  (`self.AddControllerYawInput` AxisValue))

(event `InputAxis|MoveRight`
  (params (AxisValue :type "Float (single-precision)"))
  ;[1 1 1] Charcter Movement
  (`self.AddMovementInput` (`KismetMathLibrary.GetRightVector` (`KismetMathLibrary.MakeRot` 0.0 (.yaw (`self.GetControlRotation`)))) AxisValue))

(event `InputAxis|LookUpRate`
  (params (AxisValue :type "Float (single-precision)"))
  ;[1 1 1] Gamepad Camera
  (`self.AddControllerPitchInput` (* AxisValue (`GameplayStatics.GetWorldDeltaSeconds`) (`self.BaseSpeed`))))

(event `InputAxis|LookRightRate`
  (params (AxisValue :type "Float (single-precision)"))
  ;[1 1 1] Gamepad Camera
  (`self.AddControllerYawInput` (* AxisValue (`GameplayStatics.GetWorldDeltaSeconds`) (`self.BaseSpeed`))))

(event `InputAction|Shoot`
  (bind _returnvalue (`self.K2_GetActorLocation`))
  (bind _returnvalue_2 (`self.GetControlRotation`))
  ;[1 1 1] Shoot Bullet
  (:`Pressed`
    (`|SpawnActorFromClass` "/Game/Blueprints/Bullet.Bullet_C" (`KismetMathLibrary.MakeTransform` (+ (`self.K2_GetActorLocation`) (* (`KismetMathLibrary.GetForwardVector` _returnvalue_2) 100.0)) _returnvalue_2))
    (`GameplayStatics.PlayWorldCameraShake` "/Game/Blueprints/Shake.Shake_C" _returnvalue 500.0)
    (`GameplayStatics.PlaySoundAtLocation` "/Game/StarterContent/Audio/Explosion01.Explosion01" _returnvalue)))

(event `Key|Gamepad_Special_Right`
  (:`Pressed`
    (`KismetSystemLibrary.QuitGame` (`GameplayStatics.GetPlayerController` 0) "Quit")))

(event `InputAction|Interact3`
  (bind _gamehud_widget (`self.GameHUD Widget`))
  (bind _inventory_menu (`/Game/UMG/GameHUD.Inventory Menu` _gamehud_widget))
  ;[1 1 1] Show Inventory
  (:`Pressed`
    (if (`/Game/UMG/GameHUD.InventoryActive` _gamehud_widget)
      (`/Engine/EditorBlueprintResources/StandardMacros.FlipFlop`
        (:`A`
          (`Widget.SetVisibility` _inventory_menu "Visible")
          (set `self.MenuOpen` true))
        (:`B`
          (`Widget.SetVisibility` _inventory_menu "Hidden")
          (set `self.MenuOpen` false))))))

(event `self.ReceiveBeginPlay`
  ;[1 1 1] Add GamHUD to Viewport
  (bind _returnvalue (`|CreateWidget` "/Game/UMG/GameHUD.GameHUD_C"))
  (set `self.GameHUD Widget` _returnvalue)
  ;[1 1 1] Slow Motion
  (`UserWidget.AddToViewport` _returnvalue 0))

(event `self.ReceiveTick`
  (params (DeltaSeconds :type "Float (single-precision)"))
  ;[1 1 1] Slow Motion
  (if (`self.SlowMoActive`)
    (`KismetSystemLibrary.ExecuteConsoleCommand` (`KismetStringLibrary.BuildString_Double` "" "slomo " 0.1))
    (else
      (`KismetSystemLibrary.ExecuteConsoleCommand` (`KismetStringLibrary.BuildString_Double` "" "slomo " 1.0)))))

(event `InputAction|Interact`
  ;[1 1 1] PickUp Item
  (:`Pressed`
    (if (< (`KismetArrayLibrary.Array_Length` (`/Game/UMG/GameHUD.Inventory` (`self.GameHUD Widget`))) 5)
      (`self.PickUpItem`)
      (else
        (`KismetSystemLibrary.PrintString` "InventoryFull")))))

(event `/Game/Blueprints/ActionInterface.DropAction`
  (params (InActor :type "Actor Object Reference"))
  ;[1 1 1] Drop Items
  (`self.SetActorHiddenInGame` InActor false)
  (`self.SetActorEnableCollision` InActor true)
  (`self.K2_SetActorTransform` InActor (`SceneComponent.K2_GetComponentToWorld` (`self.Drop Location`)) false))

(event `InputAction|SloMoAction`
  (bind _camera (`self.Camera`))
  (bind _camera_2 (`self.Camera`))
  ;[1 1 1] Slow Motion
  (:`Pressed`
    (set `self.SlowMoActive` true)
    ;[1 1 1] Camera Zoom
    (set `CameraComponent.FieldOfView` (`KismetMathLibrary.FClamp` (- (`CameraComponent.FieldOfView` _camera) (`self.Zoom Rate`)) (`self.CameraMin`) (`self.CameraMax`)) _camera))
  (:`Released`
    (set `self.SlowMoActive` false)
    (set `CameraComponent.FieldOfView` (`KismetMathLibrary.FClamp` (+ (`CameraComponent.FieldOfView` _camera_2) (`self.Zoom Rate`)) (`self.CameraMin`) (`self.CameraMax`)) _camera_2)))

(fn `UserConstructionScript`)
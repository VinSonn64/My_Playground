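; PlayerHUD is a HUD Blueprint that draws the collectible count and elapsed game time on screen.
; DrawHUD renders both as canvas text at fixed positions, zero-padding seconds below ten.
; AddCollectible increments the counter shown by the HUD.
; A timeline started on BeginPlay serves as the clock, supplying truncated seconds and incrementing minutes each time it finishes and restarts.
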(event `self.ReceiveDrawHUD`
  (params (SizeX :type Integer) (SizeY :type Integer))
  ;[1 1 1] Draws Collectibles on HUD
  (`self.DrawText` (`KismetStringLibrary.Concat_StrStr` "Collectibles: " (`KismetStringLibrary.Conv_IntToString` (`self.Collectibles`))) (struct :`G` 0.790925 :`B` 0.845 :`A` 1.0) 500.0 525.0 null 2.0)
  ;[1 1 1] Displays the Time
  (if (< (`self.Seconds`) 10)
    (`self.DrawText` (`KismetStringLibrary.Concat_StrStr` "GameTime    " (`KismetStringLibrary.Concat_StrStr` (`KismetStringLibrary.Concat_StrStr` (`KismetStringLibrary.Conv_IntToString` (`self.Minutes`)) ":0") (`KismetStringLibrary.Conv_IntToString` (`self.Seconds`)))) (struct :`G` 0.735071 :`B` 0.835 :`A` 1.0) 500.0 500.0 null 2.0)
    (else
      (`self.DrawText` (`KismetStringLibrary.Concat_StrStr` "GameTime    " (`KismetStringLibrary.Concat_StrStr` (`KismetStringLibrary.Concat_StrStr` (`KismetStringLibrary.Conv_IntToString` (`self.Minutes`)) ":") (`KismetStringLibrary.Conv_IntToString` (`self.Seconds`)))) (struct :`G` 0.726777 :`B` 0.82 :`A` 1.0) 500.0 500.0 null 2.0))))

(event `Add Collectible`
  ;[1 1 1] Event that adds to Colletibles
  (set `self.Collectibles` (+ (`self.Collectibles`) 1)))

(event `self.ReceiveBeginPlay`
  ;[1 1 1] Creates variables for seconds and minutes
  (bind (_direction _seconds) (`Timeline|Timeline_0` :!label _label)
    (:`Update`
      (set `self.Seconds` (`KismetMathLibrary.FTrunc` _seconds)))
    (:`Finished`
      (set `self.Minutes` (+ (`self.Minutes`) 1))
      (goto _label :!via `PlayFromStart`))))

(fn `UserConstructionScript`)
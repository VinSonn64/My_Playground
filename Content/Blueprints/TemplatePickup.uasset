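; Template pickup actor that the player collects into the HUD inventory and later uses to affect health, energy and mood.
; Construction fills its inventory struct and mesh from instance settings, and BeginPlay creates the prompt widget and binds pickup to MyCharacter.
; Trigger overlap toggles the prompt and range flag; pickup hides the actor, disables collision and refreshes the inventory.
; UseAction sets the three stats from offset Add values, then destroys the actor.
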(event `self.ReceiveBeginPlay`
  (bind _iteminfo (`self.ItemInfo`))
  (bind _pickuptextwidget (`self.PickUpTextWidget`))
  (bind (_item _itemimage _pickuptext) (break `/Game/Blueprints/InventoryStruct` _iteminfo))
  ;[1 1 1] Creats Widget and sets the info from the actors default info
  (bind _returnvalue (`|CreateWidget` "/Game/UMG/PickUpText.PickUpText_C"))
  (set `self.PickUpTextWidget` _returnvalue)
  (setmembers `/Game/Blueprints/InventoryStruct` :`StructRef` _iteminfo :`Item` self)
  ;;[1 1 1] Set The Widgets Text and Location from this Item's info
  (set `/Game/UMG/PickUpText.PickUpActor` _item _pickuptextwidget)
  (set `/Game/UMG/PickUpText.PickUpText` _pickuptext _pickuptextwidget)
  (bind _asmy_character (cast `/Game/Blueprints/MyCharacter` (`GameplayStatics.GetPlayerCharacter` 0)))
  (set `self.MyCharacter` _asmy_character)
  (add `/Game/Blueprints/MyCharacter.PickUpItem` _asmy_character (delegate `PickUpItem_Event_0`)))

(event `self.ReceiveActorBeginOverlap`
  (params (OtherActor :type "Actor Object Reference")))

(event `self.ReceiveTick`
  (params (DeltaSeconds :type "Float (single-precision)")))

(event `PickUpItem_Event_0`
  (bind _gamehud_widget (`/Game/Blueprints/MyCharacter.GameHUD Widget` (`self.MyCharacter`)))
  (if (and (`self.GetActorEnableCollision`) (`self.IsInRange`))
    ;[1 1 1] PickUp and Add to Inventory
    (`KismetArrayLibrary.Array_Add` (`/Game/UMG/GameHUD.Inventory` _gamehud_widget) (`self.ItemInfo`))
    (`Widget.RemoveFromParent` (`self.PickUpTextWidget`))
    (`self.SetActorHiddenInGame` true)
    (`self.SetActorEnableCollision` false)
    (`/Game/UMG/GameHUD.Refresh Inventory` _gamehud_widget)
    (`PrimitiveComponent.SetCollisionEnabled` (`self.Trigger`) "NoCollision")))

(event `self.Trigger.OnComponentBeginOverlap`
  (params (OtherActor :type "Actor Object Reference") (OtherComp :type "PrimitiveComponent Object Reference") (OtherBodyIndex :type Integer) (bFromSweep :type Boolean) (SweepResult :type "HitResult Structure (by ref)"))
  ;[1 1 1] Trigger
  (cast `/Game/Blueprints/MyCharacter` OtherActor)
  (`UserWidget.AddToViewport` (`self.PickUpTextWidget`) 0)
  (set `self.IsInRange` true))

(event `self.Trigger.OnComponentEndOverlap`
  (params (OtherActor :type "Actor Object Reference") (OtherComp :type "PrimitiveComponent Object Reference") (OtherBodyIndex :type Integer))
  ;[1 1 1] Trigger
  (cast `/Game/Blueprints/MyCharacter` OtherActor)
  (`Widget.RemoveFromParent` (`self.PickUpTextWidget`))
  (set `self.IsInRange` false))

(event `/Game/Blueprints/ActionInterface.UseAction`
  (bind _mycharacter (`self.MyCharacter`))
  ;[1 1 1] Item was used
  (set `/Game/Blueprints/MyCharacter.HealthValue` (+ (`self.AddHealth`) 0.5) _mycharacter)
  (set `/Game/Blueprints/MyCharacter.Energy` (+ (`self.AddEnergy`) 0.5) _mycharacter)
  (set `/Game/Blueprints/MyCharacter.Mood` (+ (`self.AddMood`) 0.5) _mycharacter)
  (`self.K2_DestroyActor`))

(fn `UserConstructionScript`
  (setmembers `/Game/Blueprints/InventoryStruct` :`StructRef` (make `/Game/Blueprints/InventoryStruct` self (`self.InventoryImage`) (`self.PickUpText`) (`self.ActionText`)))
  (`StaticMeshComponent.SetStaticMesh` (`self.Can`) (`self.CustomMesh`)))
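; Manual sliding double door Blueprint that opens when the player presses Interact inside its trigger box.
; Box overlap shows a front text prompt and enables input; leaving hides it, disables input and reverses the timeline to close the doors.
; A timeline adds left and right slide offsets to the world locations of the two door meshes stored at BeginPlay.
; Overlap events do not filter which actor triggers them.
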(event `InputAction|Interact`
  ;[1 1 1] Clicking Opens Door
  (:`Pressed`
    (bind (_direction _slidedoorr _slidedoorl) (`Timeline|Timeline_0` :!label _label)
      (:`Update`
        (`SceneComponent.K2_SetWorldLocation` (`self.SM_GlassWindow`) (+ _slidedoorr (`self.DoorLocR`)) false)
        (`SceneComponent.K2_SetWorldLocation` (`self.StaticMesh`) (+ _slidedoorl (`self.DoorLocL`)) false)))))

(event `self.Box.OnComponentEndOverlap`
  (params (OtherActor :type "Actor Object Reference") (OtherComp :type "PrimitiveComponent Object Reference") (OtherBodyIndex :type Integer))
  ;[1 1 1] Disables input and Text when leaving Trigger or opening door
  (`SceneComponent.SetVisibility` (`self.DoorFront Text`) false false)
  (`self.DisableInput` (`GameplayStatics.GetPlayerController` 0))
  (goto _label :!via `Reverse`))

(event `self.Box.OnComponentBeginOverlap`
  (params (OtherActor :type "Actor Object Reference") (OtherComp :type "PrimitiveComponent Object Reference") (OtherBodyIndex :type Integer) (bFromSweep :type Boolean) (SweepResult :type "HitResult Structure (by ref)"))
  ;[1 1 1] On Trigger Enable input and Text
  (`self.EnableInput` (`GameplayStatics.GetPlayerController` 0))
  (`SceneComponent.SetVisibility` (`self.DoorFront Text`) true false))

(event `self.ReceiveBeginPlay`
  ;[1 1 1] Store Location of Doors on Start
  (set `self.DoorLocR` (`SceneComponent.K2_GetComponentLocation` (`self.SM_GlassWindow`)))
  (set `self.DoorLocL` (`SceneComponent.K2_GetComponentLocation` (`self.StaticMesh`))))

(fn `UserConstructionScript`)
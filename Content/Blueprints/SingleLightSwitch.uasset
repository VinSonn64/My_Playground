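; SingleLightSwitch is an interactable switch actor that controls a movie and the InteractiveCeilingLight actors in the level.
; Entering its box enables player input and leaving disables it, with both overlaps toggling the visibility of two text prompts.
; Interact plays or pauses the media player through a boolean flag, while Interact2 toggles every ceiling light found by class.
; Despite the name, the logic for toggling one referenced light is unconnected.
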(event `self.ReceiveBeginPlay`)

(event `self.Box.OnComponentBeginOverlap`
  (params (OtherActor :type "Actor Object Reference") (OtherComp :type "PrimitiveComponent Object Reference") (OtherBodyIndex :type Integer) (bFromSweep :type Boolean) (SweepResult :type "HitResult Structure (by ref)"))
  ;[1 1 1] Collision enables Input and Text
  (`self.EnableInput` (`GameplayStatics.GetPlayerController` 0))
  (`SceneComponent.ToggleVisibility` (`self.TextRender`) false :!label _label)
  (`SceneComponent.ToggleVisibility` (`self.TextRender1`) false))

(event `self.ReceiveActorBeginOverlap`
  (params (OtherActor :type "Actor Object Reference")))

(event `self.ReceiveTick`
  (params (DeltaSeconds :type "Float (single-precision)")))

(event `self.Box.OnComponentEndOverlap`
  (params (OtherActor :type "Actor Object Reference") (OtherComp :type "PrimitiveComponent Object Reference") (OtherBodyIndex :type Integer))
  ;[1 1 1] Collision enables Input and Text
  (`self.DisableInput` (`GameplayStatics.GetPlayerController` 0))
  (goto _label))

(event `InputAction|Interact`
  (:`Pressed`
    ;[1 1 1] Toggle Movie
    (if (`self.IsMoviePlaying`)
      (bind _output_get (set `self.NewVar_0` "/Game/Movies/NewMediaPlayer.NewMediaPlayer"))
      (`MediaPlayer.Pause` _output_get)
      (set `self.IsMoviePlaying` false)
      (else
        (bind _output_get_2 (set `self.NewVar_0` "/Game/Movies/NewMediaPlayer.NewMediaPlayer"))
        (`MediaPlayer.Play` _output_get_2)
        (set `self.IsMoviePlaying` true)))))

(event `InputAction|Interact2`
  ;[1 1 1] Q Toggles all Light Class Actors
  (:`Pressed`
    (bind _outactors (`GameplayStatics.GetAllActorsOfClass` "/Game/Blueprints/InteractiveCeilingLight.InteractiveCeilingLight_C"))
    (for _array_element _outactors
      (bind _output_get (set `self.Light` _array_element))
      (`/Game/Blueprints/InteractiveCeilingLight.ToggleLight` _output_get))))

(fn `UserConstructionScript`)
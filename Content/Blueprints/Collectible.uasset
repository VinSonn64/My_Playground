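; Collectible pickup actor that destroys itself when anything begins overlapping its Collider, with no check on the overlapping actor.
; The overlap then calls AddCollectible on the PlayerHUD and adds a small fixed amount to player 0's MyCharacter HealthValue.
; BeginPlay caches the sphere's location for a spin-and-bob Timeline, but nothing in the graph triggers that Timeline.
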(event `self.ReceiveActorBeginOverlap`
  (params (OtherActor :type "Actor Object Reference")))

(event `self.ReceiveTick`
  (params (DeltaSeconds :type "Float (single-precision)")))

(event `self.ReceiveBeginPlay`
  (set `self.CollectibleLoc` (`SceneComponent.K2_GetComponentLocation` (`self.Sphere`))))

(event `self.Collider.OnComponentBeginOverlap`
  (params (OtherActor :type "Actor Object Reference") (OtherComp :type "PrimitiveComponent Object Reference") (OtherBodyIndex :type Integer) (bFromSweep :type Boolean) (SweepResult :type "HitResult Structure (by ref)"))
  (`self.K2_DestroyActor`)
  (bind _asplayer_hud (castclass `/Game/Blueprints/PlayerHUD` "/Game/Blueprints/PlayerHUD.PlayerHUD_C"))
  (bind _outactors (`GameplayStatics.GetAllActorsOfClass` _asplayer_hud))
  (`/Game/Blueprints/PlayerHUD.Add Collectible` _outactors)
  (bind _asmy_character (cast `/Game/Blueprints/MyCharacter` (`GameplayStatics.GetPlayerCharacter` 0)))
  (set `/Game/Blueprints/MyCharacter.HealthValue` (+ (`/Game/Blueprints/MyCharacter.HealthValue` _asmy_character) 0.1) _asmy_character))

(fn `UserConstructionScript`)